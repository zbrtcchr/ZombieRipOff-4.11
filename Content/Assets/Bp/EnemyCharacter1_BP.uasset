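; Enemy character that attacks BP-Megaman on overlap and carries a world-space health bar.
; Overlap starts a looping DamageHero timer at its attacks-per-second rate, calling the hero's AffectHealth until overlap ends.
; Its own AffectHealth stops movement, spawns floating damage text, recalculates health and destroys the actor on death.
; Tick runs Hit, which reveals, fills and rotates the health bar and clears IsDamaged after a short delay.
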(event `self.ReceiveTick`
  (params (DeltaSeconds :type "Float (single-precision)"))
  (`self.Hit`))

(event `self.ReceiveBeginPlay`
  ;[1 1 1] Initialization
  (bind _asenemy_health (cast `/Game/Assets/Bp/UI/EnemyHealth` (`WidgetComponent.GetUserWidgetObject` (`self.HealthBar`))))
  (set `self.ThisHeatlhBarUI` _asenemy_health))

(event `Hit`
  ;[1 1 1] Shows This Health BAr
  (if (not (== (`self.Health`) 100.0))
    (`SceneComponent.SetVisibility` (`self.HealthBar`) true false) ; Health Bar will show if health is less\nthan 100
  )
  (`ProgressBar.SetPercent` (`/Game/Assets/Bp/UI/EnemyHealth.ProgressBar_297` (`self.ThisHeatlhBarUI`)) (/ (`self.Health`) 100.0))
  (`SceneComponent.K2_SetWorldRotation` (`self.HealthBar`) (`self.GetPlayerInvertedRotation`) false false)
  ;[1 1 1] Sets IsDamaged back to false
  (`KismetSystemLibrary.Delay` 0.2)
  (set `self.IsDamaged` false))

(event `self.ReceiveActorBeginOverlap`
  (params (OtherActor :type "Actor Object Reference"))
  ;[1 0.1098 0.1137] Attacking, Damaging and stops attacking  Hero
  ;;[0.0902 0.003922 0.003922] Attacking Hero
  (bind _asbp_megaman (cast `/Game/Assets/Megaman/BP/BP-Megaman` OtherActor))
  (set `self.Hero` _asbp_megaman)
  (bind _returnvalue (`KismetSystemLibrary.K2_SetTimer` null "DamageHero" (/ 1.0 (`self.ThisAtacksPerSecond`)) true))
  (set `self.IsAttacking` true))

(event `/Game/Assets/Bp/iDamageable.AffectHealth`
  (params (DeltaDamage :type Integer))
  ;[1 1 1] TakingDamage
  (set `self.TakenDamage` 0)
  (`|ExecutionSequence`
    (:`then_0`
      (set `self.IsDamaged` true)
      (`MovementComponent.StopMovementImmediately` (`self.CharacterMovement`))
      ;[1 1 1] Spawns Damage Text
      (`|SpawnActorFromClass` "/Game/Assets/Bp/DamageText.DamageText_C" (`KismetMathLibrary.MakeTransform` (+ (.location (`self.GetTransform` self)) (0.0 0.0 50.0)) (`self.GetPlayerInvertedRotation`) (.scale (`self.GetTransform` self))) "Undefined" "OverrideRootScale" null (`KismetStringLibrary.Conv_IntToString` (`KismetMathLibrary.Abs_Int` (`self.TakenDamage`)))))
    (:`then_1`
      (`self.CalculateHealth` (`KismetMathLibrary.Conv_IntToDouble` (`self.TakenDamage`)))
      (if (`self.isDead`)
        (`self.K2_DestroyActor`)))))

(event `self.ReceiveActorEndOverlap`
  (params (OtherActor :type "Actor Object Reference"))
  (bind _hero (`self.Hero`))
  ;[1 0.1098 0.1137] Attacking, Damaging and stops attacking  Hero
  ;;[0.0902 0.003922 0.003922] Stopped Attacking Hero
  (if (== OtherActor _hero)
    (`KismetSystemLibrary.K2_ClearTimerHandle` (stale `self.ReceiveActorBeginOverlap` _returnvalue))
    (set `/Game/Assets/Megaman/BP/BP-Megaman.IsDamaged` false _hero)
    (set `self.IsAttacking` false)))

(event `DamageHero`
  (bind _hero (`self.Hero`))
  ;[1 0.1098 0.1137] Attacking, Damaging and stops attacking  Hero
  ;;[0.0902 0.003922 0.003922] Damaging the Hero Character by caling AffectHealth
  (`/Game/Assets/Megaman/BP/BP-Megaman.AffectHealth` _hero 0)
  (set `/Game/Assets/Megaman/BP/BP-Megaman.IsDamaged` true _hero))

(fn `UserConstructionScript`)