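; AK12_BP is an automatic rifle that spawns AK12_Projectile actors from its ProjectileSpawnPoint.
; PullTrigger fires at once, then a looping timer repeats Fire at RoundsPerSecond until ReleaseTrigger clears it and resets the DoOnce gate.
; Each shot decrements Ammo; an empty magazine blocks firing during a timed reload, then refills and deducts from MaximumAmmo without checking the remaining reserve.
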(event `PullTrigger`
  ;[1 1 1] Pulling and Releasing of trigger
  (`/Engine/EditorBlueprintResources/StandardMacros.DoOnce` false :!label _label
    (:`Completed`
      (`self.Fire`)
      (bind _returnvalue (`KismetSystemLibrary.K2_SetTimer` null "Fire" (/ 1.0 (`self.RoundsPerSecond`)) true)))))

(event `ReleaseTrigger`
  ;[1 1 1] Pulling and Releasing of trigger
  (`KismetSystemLibrary.K2_ClearTimerHandle` (stale `PullTrigger` _returnvalue))
  (goto _label :!via `Reset`))

(event `Fire`
  ;[1 1 1] Fire
  (if (`self.CanFire`)
    (`|SpawnActorFromClass` "/Game/Assets/Bp/AK12_Projectile.AK12_Projectile_C" (`SceneComponent.K2_GetComponentToWorld` (`self.ProjectileSpawnPoint`)) "Undefined" "OverrideRootScale")
    (set `self.Ammo` (- (`self.Ammo`) 1))
    (`self.CalculateAmmo`)))

(event `CalculateAmmo`
  ;[1 1 1] Computes for amount of remaining ammo
  (if (<= (`self.Ammo`) 0)
    (set `self.CanFire` false)
    (`KismetSystemLibrary.Delay` 3.0)
    (bind _output_get (set `self.Ammo` 50))
    (set `self.MaximumAmmo` (- (`self.MaximumAmmo`) _output_get))
    (set `self.CanFire` true)))

(fn `UserConstructionScript`)